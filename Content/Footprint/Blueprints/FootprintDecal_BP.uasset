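; Footprint decal actor that stays for a set lifetime, fades out, then destroys itself.
; BeginPlay creates a dynamic material instance on the decal and starts a lifetime timer, which chains into a fade timer that ends in DestroyActor.
; Tick drives the material's Fade scalar as one minus the fade timer's elapsed fraction, so the timer handle doubles as the animation clock.
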(event `self.ReceiveTick`
  (params (DeltaSeconds :type "Float (single-precision)"))
  (`MaterialInstanceDynamic.SetScalarParameterValue` (stale `self.ReceiveBeginPlay` _returnvalue) "Fade" (- 1.0 (/ (`KismetSystemLibrary.K2_GetTimerElapsedTimeHandle` (stale `BeginFade` _returnvalue)) (`self.FadeTime`))) :!label _label))

(event `self.ReceiveBeginPlay`
  (`KismetSystemLibrary.K2_SetTimerDelegate` (delegate `BeginFade`) (`self.LifeTime`))
  (bind _returnvalue (`DecalComponent.CreateDynamicMaterialInstance` (`self.Decal`)))
  (goto _label))

(event `BeginFade`
  (bind _returnvalue (`KismetSystemLibrary.K2_SetTimerDelegate` (delegate `DestroyFootprint`) (`self.FadeTime`))))

(event `DestroyFootprint`
  (`self.K2_DestroyActor`))

(fn `UserConstructionScript`)