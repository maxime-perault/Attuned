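; Third-person camera manager that drives the player's spring arm and follow camera for pitch framing, obstruction avoidance and water transitions.
; A water timeline scales max arm length and steers control rotation on entry.
; Pitch scrubs the PeriphVision timeline as a lookup for arm length, boom height and FOV.
; Camera-channel traces, backed by sphere overlap and Visibility traces, pull the camera in instantly, while another timeline eases it back out.
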(event `self.ReceiveBeginPlay`
  (bind _asbp_third_person_character (cast `/Game/Attuned/Characters/Player/MainCharacter/Blueprints/BP_ThirdPersonCharacter` (`GameplayStatics.GetPlayerPawn` 0)))
  (bind _output_get (set `self.ThirdPerson` _asbp_third_person_character))
  (set `self.FollowCamera` (`/Game/Attuned/Characters/Player/MainCharacter/Blueprints/BP_ThirdPersonCharacter.FollowCamera` _output_get))
  (set `self.CameraBoom` (`/Game/Attuned/Characters/Player/MainCharacter/Blueprints/BP_ThirdPersonCharacter.CameraBoom` _output_get))
  (set `self.CameraCollision` (`/Game/Attuned/Characters/Player/MainCharacter/Blueprints/BP_ThirdPersonCharacter.CameraCollision` _output_get))
  (set `self.BaseCameraBoomZ` (.z (`SceneComponent.RelativeLocation` (`self.CameraBoom`))))
  (set `self.DeltaCameraBoomZ` 40.0)
  (set `self.BaseFOV` 90.0)
  (set `self.DeltaFOV` 10.0)
  (set `self.CurrentPitch` 0.0)
  (bind _output_get_2 (set `self.MaxArmLength` (`SpringArmComponent.TargetArmLength` (`self.CameraBoom`))))
  (bind _output_get_3 (set `self.LastResArmLength` _output_get_2))
  (bind _output_get_4 (set `self.ArmLengthMaxFromPitch` _output_get_3))
  (bind _output_get_5 (set `self.BaseMaxArmLength` _output_get_4))
  (set `self.DeltaMaxArmLength` 200.0)
  ;[1 1 1] ArmLength - Sphere collision radius
  (`self.SetCameraArmLength` _output_get_5))

(event `self.ReceiveTick`
  (params (DeltaSeconds :type "Float (single-precision)"))
  (bind _cameratransitions (`self.CameraTransitions`))
  (bind _cameratransitions_2 (`self.CameraTransitions`))
  (bind _returnvalue (`SceneComponent.K2_GetComponentLocation` (`self.CameraBoom`)))
  (bind _returnvalue_2 (- (`self.MaxArmLength`) (`SphereComponent.SphereRadius` (`self.CameraCollision`))))
  ;[1 1 1] Water transition for the camera
  (if (`self.transitionCameraInWater`)
    (if (or (`TimelineComponent.IsReversing` _cameratransitions) (not (`TimelineComponent.IsPlaying` _cameratransitions)))
      (bind (_direction _scale) (`Timeline|CameraTransitions` :!label _label)
        (:`Update`
          (set `self.MaxArmLength` (+ (`self.BaseMaxArmLength`) (* _scale (`self.DeltaMaxArmLength`))))
          (`/Game/Attuned/Characters/Player/MainCharacter/Blueprints/BP_ThirdPersonCharacter.DebugTextLocation` (`self.ThirdPerson`))
          (if (`self.transitionCameraInWater`)
            (`Controller.SetControlRotation` (`GameplayStatics.GetPlayerController` 0) (`KismetMathLibrary.MakeRotator` (.roll (`KismetMathLibrary.RLerp` (`KismetMathLibrary.MakeRotator` 0.0 (.pitch (`self.BaseControlRotator`)) (.yaw (`self.BaseControlRotator`))) (`KismetMathLibrary.MakeRotator` 0.0 -5.0 (.yaw (`self.BasePlayerRotator`))) _scale true)) (.pitch (`KismetMathLibrary.RLerp` (`KismetMathLibrary.MakeRotator` 0.0 (.pitch (`self.BaseControlRotator`)) (.yaw (`self.BaseControlRotator`))) (`KismetMathLibrary.MakeRotator` 0.0 -5.0 (.yaw (`self.BasePlayerRotator`))) _scale true)) (+ (.yaw (`KismetMathLibrary.RLerp` (`KismetMathLibrary.MakeRotator` 0.0 (.pitch (`self.BaseControlRotator`)) (.yaw (`self.BaseControlRotator`))) (`KismetMathLibrary.MakeRotator` 0.0 -5.0 (.yaw (`self.BasePlayerRotator`))) _scale true)) (`self.DeltaRotCameraWater`))))))
        (:`Finished`
          (set `self.transitionCameraOutWater` false)
          (set `self.transitionCameraInWater` false)
          (`Controller.SetControlRotation` (`GameplayStatics.GetPlayerController` 0) (`KismetMathLibrary.MakeRotator` 0.0 (.pitch (`Pawn.GetControlRotation` (`GameplayStatics.GetPlayerPawn` 0))) (.yaw (`Pawn.GetControlRotation` (`GameplayStatics.GetPlayerPawn` 0)))))))
      ;[1 1 1] Camera settings, dont forget to check "can generate overlap events" on each element which can interact with the camera
      (`/Game/Attuned/Characters/Player/MainCharacter/Blueprints/BP_ThirdPersonCharacter.CheckAICamControl` (`self.ThirdPerson`) :!label _label_2)
      ;;[1 1 1] Get the Max Arm Length depending of the pitch (the -1;1 pitch value is now a 0;2 range to get the value on a timeline)
      (bind _result (`/Engine/EditorBlueprintResources/StandardMacros.IncrementFloat` (/ (- (.z (- (`SceneComponent.K2_GetComponentLocation` (`self.CameraBoom`)) (* (`KismetMathLibrary.Normal` (`KismetMathLibrary.GetForwardVector` (`SceneComponent.K2_GetComponentRotation` (`self.FollowCamera`)))) _returnvalue_2))) (.z (`SceneComponent.K2_GetComponentLocation` (`self.CameraBoom`)))) _returnvalue_2))
        (:`  `
          (bind _output_get (set `self.CurrentPitch` _result))
          (bind (_direction_2 _maxarmlengthscale _deltacameraboomz) (`Timeline|PeriphVision` :`NewTime` _output_get :!via `SetNewTime`)
            (:`Update`
              (set `self.ArmLengthMaxFromPitch` (* _maxarmlengthscale (`self.MaxArmLength`)))
              (`SceneComponent.K2_SetRelativeLocation` (`self.CameraBoom`) (`KismetMathLibrary.MakeVector` 0.0 0.0 (+ (* (`self.DeltaCameraBoomZ`) _deltacameraboomz) (`self.BaseCameraBoomZ`))) false false)
              (`CameraComponent.SetFieldOfView` (`self.FollowCamera`) (+ (`self.BaseFOV`) (* _deltacameraboomz (`self.DeltaFOV`))))
              (bind _output_get_2 (set `self.FakeCameraFromMaxLength` (- _returnvalue (* (`KismetMathLibrary.Normal` (`KismetMathLibrary.GetForwardVector` (`SceneComponent.K2_GetComponentRotation` (`self.FollowCamera`)))) (`self.ArmLengthMaxFromPitch`)))))
              (bind _outhit (`KismetSystemLibrary.LineTraceSingle` _returnvalue _output_get_2 "TraceTypeQuery2"))
              (bind _output_get_3 (set `self.CameraPlayerDistance` (`.Distance` (`GameplayStatics.BreakHitResult` _outhit))))
              ;;[1 1 1] Force New Arm lenght if there is something between the character and the Camera
              (if (and (> _output_get_3 0.0) (< _output_get_3 (`self.ArmLengthMaxFromPitch`)))
                ;;;[1 1 1] One element between Camera and player found, force new arm length
                (bind _output_get_4 (set `self.ResArmLength` (`self.CameraPlayerDistance`)))
                (if (or (and (`self.IsZoomingOut`) (> (`self.LastResArmLength`) _output_get_4)) (not (`self.IsZoomingOut`)))
                  (`self.SetCameraArmLength` _output_get_4 true)
                  (else
                    ;;[1 1 1] ZOOM OUT
                    ;;;[1 1 1] No collision detected.
                    ;;; Set Standard Arm lenght with a Zoom Out.
                    ;;; (Play timeline only if possible)
                    (if (and (and (not (`TimelineComponent.IsPlaying` (`self.ScalingPushOutCamera`))) (!= (`self.ResArmLength`) (`self.ArmLengthMaxFromPitch`))) (`self.IsZoomingOut`)) :!label _label_3
                      ;;;[1 1 1] Set New Time for Timeline Start Depending of the last arm Length
                      (`TimelineComponent.SetNewTime` (`self.ScalingPushOutCamera`) (* (/ (`self.ResArmLength`) (`self.ArmLengthMaxFromPitch`)) (`TimelineComponent.GetTimelineLength` (`self.ScalingPushOutCamera`))))
                      ;;;[1 1 1] Length: 2sec // Scaling Timeline from last arm lenght to standard arm length
                      (bind (_direction_3 _scale_2) (`Timeline|ScalingPushOutCamera`)
                        (:`Update`
                          (bind _returnvalue_3 (* _scale_2 (`self.ArmLengthMaxFromPitch`)))
                          (`self.SetCameraArmLength` _returnvalue_3 true)
                          (bind _output_get_5 (set `self.ResArmLength` _returnvalue_3))
                          (set `self.LastResArmLength` _output_get_5))
                        (:`Finished`
                          (set `self.IsZoomingOut` false)
                          (set `self.LastResArmLength` (`self.ArmLengthMaxFromPitch`))))
                      (else
                        ;;;[1 1 1] Set Camera Arm Length depending of the pitch
                        (if (not (`TimelineComponent.IsPlaying` (`self.ScalingPushOutCamera`)))
                          (`self.SetCameraArmLength` (`self.ArmLengthMaxFromPitch`)))))))
                (else
                  (`SceneComponent.K2_SetWorldLocation` (`self.CameraCollision`) (`self.FakeCameraFromMaxLength`) false false)
                  ;;[1 1 1] Check collision with camera
                  (if (> (`KismetArrayLibrary.Array_Length` (`PrimitiveComponent.GetOverlappingActors` (`self.CameraCollision`) null)) 0)
                    ;;[1 1 1] Check Visible Chan now, because the camera is inside something not catchable in camera chan
                    (bind _outhit_2 (`KismetSystemLibrary.LineTraceSingle` (`SceneComponent.K2_GetComponentLocation` (`self.CameraBoom`)) (`self.FakeCameraFromMaxLength`) "TraceTypeQuery1"))
                    (bind _output_get_6 (set `self.CameraPlayerDistance` (`.Distance` (`GameplayStatics.BreakHitResult` _outhit_2))))
                    (if (!= _output_get_6 0.0)
                      (bind _output_get_7 (set `self.ResArmLength` _output_get_6))
                      (if (or (and (`self.IsZoomingOut`) (> (`self.LastResArmLength`) _output_get_7)) (not (`self.IsZoomingOut`)))
                        (`self.SetCameraArmLength` _output_get_6 true)
                        (else
                          (goto _label_3)))
                      (else
                        (goto _label_3)))
                    (else
                      (goto _label_3))))))))))
    (elif (`self.transitionCameraOutWater`)
      (if (or (not (`TimelineComponent.IsReversing` _cameratransitions_2)) (not (`TimelineComponent.IsPlaying` _cameratransitions_2)))
        (goto _label :!via `Reverse`))
      (else
        (goto _label_2)))))

(fn `SetCameraArmLength`
  (params (CameraDistance :type "Float (double-precision)") (PushIn :type Boolean))
  (bind _output_get (set `SpringArmComponent.TargetArmLength` (- CameraDistance (`SphereComponent.GetScaledSphereRadius` (`self.CameraCollision`))) (`self.CameraBoom`)))
  (set `self.LastResArmLength` _output_get)
  (if PushIn
    (`TimelineComponent.Stop` (`self.ScalingPushOutCamera`))
    (set `self.IsZoomingOut` true)))

(fn `UserConstructionScript`)