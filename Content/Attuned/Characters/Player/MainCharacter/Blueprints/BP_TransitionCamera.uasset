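; Camera actor that moves the player's view between the third-person character and the menu.
; SwitchCamera sets the view target to itself or the character, either instantly when forced or blended over BlendTime, locking controls and toggling UIMenu.
; For blends, a timeline sized to BlendTime in the construction script acts as a wait, blocking repeat switches.
; When it finishes, it flips MvMenu, shows the menu or unlocks controls, and clears TransitionCamLock.
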(event `self.ReceiveBeginPlay`
  (bind _asbp_cppthird_person_character (cast `/Game/Attuned/Characters/Player/MainCharacter/Blueprints/BP_CPPThirdPersonCharacter` (`GameplayStatics.GetPlayerCharacter` 0)))
  (set `self.ThirdPerson` _asbp_cppthird_person_character))

(event `StartTimeline`
  (bind _thirdperson (`self.ThirdPerson`))
  (`Timeline|WaitCameraTransition` :!via `PlayFromStart`
    (:`Finished`
      (if (`MyCharacter.mv_Menu` _thirdperson)
        (`MyCharacter.UnlockControls` _thirdperson)
        (set `MyCharacter.mv_Menu` false (`self.ThirdPerson`))
        (else
          (`Widget.SetVisibility` (`/Game/Attuned/Characters/Player/MainCharacter/Blueprints/BP_CPPThirdPersonCharacter.UI_Menu` _thirdperson) "Visible")
          (set `MyCharacter.mv_Menu` true (`self.ThirdPerson`))))
      (set `/Game/Attuned/Characters/Player/MainCharacter/Blueprints/BP_CPPThirdPersonCharacter.TransitionCamLock` false (`self.ThirdPerson`)))))

(fn `SwitchCamera`
  (params (`Switch From TPS To Menu` :type Boolean) (ForceSwitch :type Boolean))
  (if `Switch From TPS To Menu`
    (if ForceSwitch
      (`PlayerController.SetViewTargetWithBlend` (`GameplayStatics.GetPlayerController` 0) self 0.0 "VTBlend_Linear" 0.0 false)
      (bind _asbp_cppthird_person_character (cast `/Game/Attuned/Characters/Player/MainCharacter/Blueprints/BP_CPPThirdPersonCharacter` (`GameplayStatics.GetPlayerCharacter` 0)))
      (`Widget.SetVisibility` (`/Game/Attuned/Characters/Player/MainCharacter/Blueprints/BP_CPPThirdPersonCharacter.UI_Menu` _asbp_cppthird_person_character) "Visible")
      (`MyCharacter.lockControls` _asbp_cppthird_person_character)
      (set `MyCharacter.mv_Menu` true (`self.ThirdPerson`))
      (elif (not (`TimelineComponent.IsPlaying` (`self.WaitCameraTransition`)))
        (`PlayerController.SetViewTargetWithBlend` (`GameplayStatics.GetPlayerController` 0) self (`self.BlendTime`) "VTBlend_Cubic" 0.0 false)
        (bind _asbp_cppthird_person_character_2 (cast `/Game/Attuned/Characters/Player/MainCharacter/Blueprints/BP_CPPThirdPersonCharacter` (`GameplayStatics.GetPlayerCharacter` 0)))
        (`MyCharacter.lockControls` _asbp_cppthird_person_character_2)
        (set `/Game/Attuned/Characters/Player/MainCharacter/Blueprints/BP_CPPThirdPersonCharacter.TransitionCamLock` true (`self.ThirdPerson`) :!label _label)
        (`self.StartTimeline`)))
    (elif ForceSwitch
      (`PlayerController.SetViewTargetWithBlend` (`GameplayStatics.GetPlayerController` 0) (`GameplayStatics.GetPlayerCharacter` 0) 0.0 "VTBlend_Linear" 0.0 false)
      (bind _asbp_cppthird_person_character_3 (cast `/Game/Attuned/Characters/Player/MainCharacter/Blueprints/BP_CPPThirdPersonCharacter` (`GameplayStatics.GetPlayerCharacter` 0)))
      (`Widget.SetVisibility` (`/Game/Attuned/Characters/Player/MainCharacter/Blueprints/BP_CPPThirdPersonCharacter.UI_Menu` _asbp_cppthird_person_character_3) "Hidden")
      (`MyCharacter.UnlockControls` _asbp_cppthird_person_character_3)
      (set `MyCharacter.mv_Menu` false (`self.ThirdPerson`))
      (elif (not (`TimelineComponent.IsPlaying` (`self.WaitCameraTransition`)))
        (`PlayerController.SetViewTargetWithBlend` (`GameplayStatics.GetPlayerController` 0) (`GameplayStatics.GetPlayerCharacter` 0) (`self.BlendTime`) "VTBlend_Linear" 0.0 false)
        (bind _asbp_cppthird_person_character_4 (cast `/Game/Attuned/Characters/Player/MainCharacter/Blueprints/BP_CPPThirdPersonCharacter` (`GameplayStatics.GetPlayerCharacter` 0)))
        (`Widget.SetVisibility` (`/Game/Attuned/Characters/Player/MainCharacter/Blueprints/BP_CPPThirdPersonCharacter.UI_Menu` _asbp_cppthird_person_character_4) "Hidden")
        (goto _label)))))

(fn `UserConstructionScript`
  (`TimelineComponent.SetTimelineLength` (`self.WaitCameraTransition`) (`self.BlendTime`)))