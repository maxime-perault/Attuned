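; BP_DestructibleBlock is a breakable grey block that reacts once when its destructible mesh first fractures.
; On that fracture the mesh stops colliding with Pawn and Destructible channels, and a radial force component fires an impulse to scatter the pieces.
; It also plays a Wwise rock explosion sound at the block's location and sends a short force feedback rumble to the first player's controller.
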(event `self.AD_Cube_DM.OnComponentFracture`
  (params (HitPoint :type "Vector Structure (by ref)") (HitDirection :type "Vector Structure (by ref)"))
  (bind _ad_cube_dm (`self.AD_Cube_DM`))
  (if (not (`self.firstTrigger`))
    (set `self.firstTrigger` true)
    (`PrimitiveComponent.SetCollisionResponseToChannel` _ad_cube_dm "ECC_Pawn" "ECR_Ignore")
    (`PrimitiveComponent.SetCollisionResponseToChannel` _ad_cube_dm "ECC_Destructible" "ECR_Ignore")
    (`RadialForceComponent.FireImpulse` (`self.RadialForce`))
    (`AkGameplayStatics.PostEventAtLocation` "/Game/Wwise/S_SFX_Explosion_Rock.S_SFX_Explosion_Rock" (`SceneComponent.K2_GetComponentLocation` (`self.DefaultSceneRoot`)) (`SceneComponent.K2_GetComponentRotation` (`Character.CapsuleComponent` (`GameplayStatics.GetPlayerCharacter` 0))))
    (`PlayerController.PlayDynamicForceFeedback` (`GameplayStatics.GetPlayerController` 0) 1.0 0.3 true true true true)))

(fn `UserConstructionScript`)