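; BP_DestructibleBlock_2 is a one-shot destructible rock block, set off when the player character's capsule overlaps its Trigger or when its destructible mesh fractures.
; Both paths share one sequence guarded by FirstTrigger, though the overlap path also waits for BeginPlay initialization.
; That sequence fires a radial impulse, makes the debris ignore Pawns, posts a Wwise rock explosion sound and plays controller force feedback.
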(event `self.ReceiveBeginPlay`
  (bind _asbp_cppthird_person_character (cast `/Game/Attuned/Characters/Player/MainCharacter/Blueprints/BP_CPPThirdPersonCharacter` (`GameplayStatics.GetPlayerCharacter` 0)))
  (set `self.ThirdPerson` _asbp_cppthird_person_character)
  (set `self.Initialized` true))

(event `self.Trigger.OnComponentBeginOverlap`
  (params (OverlappedComponent :type "PrimitiveComponent Object Reference") (OtherActor :type "Actor Object Reference") (OtherComp :type "PrimitiveComponent Object Reference") (OtherBodyIndex :type Integer) (bFromSweep :type Boolean) (SweepResult :type "HitResult Structure (by ref)"))
  (bind _debris_03_dm (`self.Debris_03_DM`))
  (if (`self.Initialized`)
    (if (and (and (== (`GameplayStatics.GetObjectClass` OtherComp) "/Script/Engine.CapsuleComponent") (== (`GameplayStatics.GetObjectClass` OtherActor) "/Game/Attuned/Characters/Player/MainCharacter/Blueprints/BP_CPPThirdPersonCharacter.BP_CPPThirdPersonCharacter_C")) (== (`self.firstTrigger`) false))
      (set `self.firstTrigger` true :!label _label)
      (`RadialForceComponent.FireImpulse` (`self.RadialForce`))
      (`PrimitiveComponent.SetCollisionObjectType` _debris_03_dm "ECC_GameTraceChannel1")
      (`PrimitiveComponent.SetCollisionResponseToChannel` _debris_03_dm "ECC_Pawn" "ECR_Ignore")
      (`AkGameplayStatics.PostEventAtLocation` "/Game/Wwise/S_SFX_Explosion_Rock.S_SFX_Explosion_Rock" (`SceneComponent.K2_GetComponentLocation` (`self.DefaultSceneRoot`)) (`SceneComponent.K2_GetComponentRotation` (`Character.CapsuleComponent` (`GameplayStatics.GetPlayerCharacter` 0))))
      (`PlayerController.PlayDynamicForceFeedback` (`GameplayStatics.GetPlayerController` 0) 1.0 0.3 true true true true))))

(event `self.Caillou_LP_DM.OnComponentFracture`
  (params (HitPoint :type "Vector Structure (by ref)") (HitDirection :type "Vector Structure (by ref)"))
  (if (== (`self.firstTrigger`) false)
    (goto _label)))

(fn `UserConstructionScript`)