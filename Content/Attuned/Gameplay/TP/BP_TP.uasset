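; BP_TP is a one-shot teleport trigger that moves the player character to a set destination.
; When a BP_CPPThirdPersonCharacter's capsule first overlaps the Trigger component, it sets a Triggered flag so later overlaps are ignored.
; It then teleports player 0's character, rather than the overlapping actor reference, to the Position component's world location without sweeping.
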(event `self.Trigger.OnComponentBeginOverlap`
  (params (OverlappedComponent :type "PrimitiveComponent Object Reference") (OtherActor :type "Actor Object Reference") (OtherComp :type "PrimitiveComponent Object Reference") (OtherBodyIndex :type Integer) (bFromSweep :type Boolean) (SweepResult :type "HitResult Structure (by ref)"))
  (if (and (and (== (`GameplayStatics.GetObjectClass` OtherComp) "/Script/Engine.CapsuleComponent") (== (`GameplayStatics.GetObjectClass` OtherActor) "/Game/Attuned/Characters/Player/MainCharacter/Blueprints/BP_CPPThirdPersonCharacter.BP_CPPThirdPersonCharacter_C")) (== (`self.Triggered`) false))
    (set `self.Triggered` true)
    (bind _asbp_cppthird_person_character (cast `/Game/Attuned/Characters/Player/MainCharacter/Blueprints/BP_CPPThirdPersonCharacter` (`GameplayStatics.GetPlayerCharacter` 0)))
    (`self.K2_SetActorLocation` _asbp_cppthird_person_character (`SceneComponent.K2_GetComponentLocation` (`self.Position`)) false true)))

(fn `UserConstructionScript`)