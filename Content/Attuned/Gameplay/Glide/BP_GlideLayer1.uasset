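; Glide trigger volume that starts the first percussion layer of the game's Wwise audio.
; On BeginPlay it sets all three percussion layer state groups to inactive.
; The first time the third-person character's capsule overlaps the Box, it posts the Play_Glide event on the player and switches Layer 01 to active, latched by a Triggered flag so it fires only once.
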(event `self.ReceiveBeginPlay`
  (`AkGameplayStatics.SetState` "Percu_Layer_01" "Inactive_01")
  (`AkGameplayStatics.SetState` "Percu_Layer_02" "Inactive_02")
  (`AkGameplayStatics.SetState` "Percu_Layer_03" "Inactive_03"))

(event `self.Box.OnComponentBeginOverlap`
  (params (OverlappedComponent :type "PrimitiveComponent Object Reference") (OtherActor :type "Actor Object Reference") (OtherComp :type "PrimitiveComponent Object Reference") (OtherBodyIndex :type Integer) (bFromSweep :type Boolean) (SweepResult :type "HitResult Structure (by ref)"))
  (if (and (and (== (`GameplayStatics.GetObjectClass` OtherComp) "/Script/Engine.CapsuleComponent") (== (`GameplayStatics.GetObjectClass` OtherActor) "/Game/Attuned/Characters/Player/MainCharacter/Blueprints/BP_CPPThirdPersonCharacter.BP_CPPThirdPersonCharacter_C")) (== (`self.Triggered`) false))
    (set `self.Triggered` true)
    (`AkGameplayStatics.PostEvent` "/Game/Wwise/Play_Glide.Play_Glide" (`GameplayStatics.GetPlayerCharacter` 0))
    (`AkGameplayStatics.SetState` "Percu_Layer_01" "Active_01")))

(fn `UserConstructionScript`)