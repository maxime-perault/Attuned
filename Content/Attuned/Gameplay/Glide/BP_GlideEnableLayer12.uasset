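; BP_GlideEnableLayer12 is a one-shot overlap trigger in the Glide gameplay folder that switches on percussion layers 1 and 2 of the audio.
; When an overlapping actor's class is exactly BP_CPPThirdPersonCharacter, it sets the Percu_Layer_01 and Percu_Layer_02 state groups to their active states through Wwise-style SetState calls.
; A Triggered flag blocks repeat firing, and nothing here resets the states.
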(event `self.ReceiveActorBeginOverlap`
  (params (OtherActor :type "Actor Object Reference"))
  (set `self.Actor` OtherActor)
  (if (and (== (`GameplayStatics.GetObjectClass` (`self.Actor`)) "/Game/Attuned/Characters/Player/MainCharacter/Blueprints/BP_CPPThirdPersonCharacter.BP_CPPThirdPersonCharacter_C") (not (`self.Triggered`)))
    (set `self.Triggered` true)
    (`AkGameplayStatics.SetState` "Percu_Layer_01" "Active_01")
    (`AkGameplayStatics.SetState` "Percu_Layer_02" "Active_02")))

(fn `UserConstructionScript`)