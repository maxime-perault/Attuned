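; Corridor trigger actor that applies a low-pass audio effect while the player character is inside its LowPassTrigger volume.
; Begin and end overlaps respond only to the third-person character's capsule, with a Triggered flag blocking repeated calls.
; Each sets the Wwise Low_Pass RTPC on the player pawn, interpolating it up on entry and back to zero on exit.
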(event `self.LowPassTrigger.OnComponentBeginOverlap`
  (params (OverlappedComponent :type "PrimitiveComponent Object Reference") (OtherActor :type "Actor Object Reference") (OtherComp :type "PrimitiveComponent Object Reference") (OtherBodyIndex :type Integer) (bFromSweep :type Boolean) (SweepResult :type "HitResult Structure (by ref)"))
  ;[1 1 1] Reverb On
  (if (and (and (== (`GameplayStatics.GetObjectClass` OtherActor) "/Game/Attuned/Characters/Player/MainCharacter/Blueprints/BP_CPPThirdPersonCharacter.BP_CPPThirdPersonCharacter_C") (== (`GameplayStatics.GetObjectClass` OtherComp) "/Script/Engine.CapsuleComponent")) (not (`self.Triggered`)))
    (set `self.Triggered` true)
    (bind _asbp_cppthird_person_character (cast `/Game/Attuned/Characters/Player/MainCharacter/Blueprints/BP_CPPThirdPersonCharacter` (`GameplayStatics.GetPlayerPawn` 0)))
    (`AkGameplayStatics.SetRTPCValue` "Low_Pass" 0.8 1000 _asbp_cppthird_person_character)))

(event `self.LowPassTrigger.OnComponentEndOverlap`
  (params (OverlappedComponent :type "PrimitiveComponent Object Reference") (OtherActor :type "Actor Object Reference") (OtherComp :type "PrimitiveComponent Object Reference") (OtherBodyIndex :type Integer))
  ;[1 1 1] Reverb Off
  (if (and (and (== (`GameplayStatics.GetObjectClass` OtherActor) "/Game/Attuned/Characters/Player/MainCharacter/Blueprints/BP_CPPThirdPersonCharacter.BP_CPPThirdPersonCharacter_C") (== (`GameplayStatics.GetObjectClass` OtherComp) "/Script/Engine.CapsuleComponent")) (`self.Triggered`))
    (set `self.Triggered` false)
    (bind _asbp_cppthird_person_character (cast `/Game/Attuned/Characters/Player/MainCharacter/Blueprints/BP_CPPThirdPersonCharacter` (`GameplayStatics.GetPlayerPawn` 0)))
    (`AkGameplayStatics.SetRTPCValue` "Low_Pass" 0.0 1000 _asbp_cppthird_person_character)))

(fn `UserConstructionScript`)