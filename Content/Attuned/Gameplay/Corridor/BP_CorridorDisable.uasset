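; BP_CorridorDisable is a one-shot trigger volume in the Corridor gameplay set that silences the music, whisper and singing audio.
; The first box overlap by the capsule of a BP_CPPThirdPersonCharacter latches a Triggered flag.
; It then sets the Wwise Music state to None, posts the whisper stop event and posts four sing stop events on every ImmortalSing actor in the level.
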(event `self.Box.OnComponentBeginOverlap`
  (params (OverlappedComponent :type "PrimitiveComponent Object Reference") (OtherActor :type "Actor Object Reference") (OtherComp :type "PrimitiveComponent Object Reference") (OtherBodyIndex :type Integer) (bFromSweep :type Boolean) (SweepResult :type "HitResult Structure (by ref)"))
  (if (and (and (== (`GameplayStatics.GetObjectClass` OtherComp) "/Script/Engine.CapsuleComponent") (== (`GameplayStatics.GetObjectClass` OtherActor) "/Game/Attuned/Characters/Player/MainCharacter/Blueprints/BP_CPPThirdPersonCharacter.BP_CPPThirdPersonCharacter_C")) (== (`self.Triggered`) false))
    (set `self.Triggered` true)
    (`AkGameplayStatics.SetState` "Music")
    (`AkGameplayStatics.PostEvent` "/Game/Wwise/Stop_Whisper.Stop_Whisper")
    (bind _outactors (`GameplayStatics.GetAllActorsOfClass` "/Game/Attuned/Gameplay/Sounds/ImmortalSing.ImmortalSing_C"))
    (for _array_element _outactors
      (`AkGameplayStatics.PostEvent` "/Game/Wwise/Stop_Sing_01.Stop_Sing_01" _array_element)
      (`AkGameplayStatics.PostEvent` "/Game/Wwise/Stop_Sing_02.Stop_Sing_02" _array_element)
      (`AkGameplayStatics.PostEvent` "/Game/Wwise/Stop_Sing_03.Stop_Sing_03" _array_element)
      (`AkGameplayStatics.PostEvent` "/Game/Wwise/Stop_Sing_04.Stop_Sing_04" _array_element))))

(fn `UserConstructionScript`)