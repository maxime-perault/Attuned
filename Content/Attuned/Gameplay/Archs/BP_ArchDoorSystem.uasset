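; Arch puzzle door that opens once every arch in its Archs array is triggered.
; Tick checks the arches until all pass, then latches, launches the ArchSystemCameraResolution cinematic and switches the Wwise music state.
; A timeline lowers the chained platforms with a chain sound, and on finish a second timeline raises the door with an open sound.
; Both movements offset cached world locations on Z by ZDelta.
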(event `self.ReceiveTick`
  (params (DeltaSeconds :type "Float (single-precision)"))
  (if (not (`self.SystemTriggered`))
    (set `self.SuccessLoop` false)
    (for (_array_element _array_index) (`self.Archs`)
      (if (`/Game/Attuned/Gameplay/Archs/BP_Arch.Triggered` _array_element)
        (if (== (- (`KismetArrayLibrary.Array_Length` (`self.Archs`)) 1) _array_index)
          (set `self.SuccessLoop` true))
        (else
          (break))))
    (if (`self.SuccessLoop`)
      (set `self.SystemTriggered` true)
      (bind _outactors (`GameplayStatics.GetAllActorsOfClass` "/Game/Attuned/Gameplay/Archs/ArchSystemCameraResolution.ArchSystemCameraResolution_C"))
      (`/Game/Attuned/Gameplay/Archs/ArchSystemCameraResolution.LaunchCinematic` (`|GetArrayItem` _outactors))
      (set `self.DoorBaseLocation` (`SceneComponent.K2_GetComponentLocation` (`self.DoorPlaceOlder(Modified Scale)`)))
      (for _array_element_2 (`self.ChainedPlatforms`)
        (`KismetArrayLibrary.Array_Add` (`self.ChainedPlatformsBaseLocation`) (`SceneComponent.K2_GetComponentLocation` (`/Game/Attuned/Gameplay/Archs/BP_ChainedPlatform.DefaultSceneRoot` _array_element_2))))
      (`AkGameplayStatics.PostEventAtLocation` "/Game/Wwise/S_SFX_Door_Chains.S_SFX_Door_Chains" (`|GetArrayItem` (`self.ChainedPlatformsBaseLocation`)))
      (`AkGameplayStatics.SetState` "Music" "Cinematique_Door")
      (bind (_direction _newtrack_0) (`Timeline|TranslatePlatforms` :!via `PlayFromStart`)
        (:`Update`
          (for (_array_element_3 _array_index_2) (`self.ChainedPlatforms`)
            (`SceneComponent.K2_SetWorldLocation` (`/Game/Attuned/Gameplay/Archs/BP_ChainedPlatform.DefaultSceneRoot` _array_element_3) (`KismetMathLibrary.MakeVector` (.x (`|GetArrayItem` (`self.ChainedPlatformsBaseLocation`) _array_index_2)) (.y (`|GetArrayItem` (`self.ChainedPlatformsBaseLocation`) _array_index_2)) (- (.z (`|GetArrayItem` (`self.ChainedPlatformsBaseLocation`) _array_index_2)) (* (`self.ZDelta`) _newtrack_0))) false false)))
        (:`Finished`
          (`AkGameplayStatics.PostEventAtLocation` "/Game/Wwise/S_SFX_Door_Open.S_SFX_Door_Open" (`SceneComponent.K2_GetComponentLocation` (`self.DoorFrame`)))
          (bind (_direction_2 _newtrack_0_2) (`Timeline|TranslateDoor` :!via `PlayFromStart`)
            (:`Update`
              (`SceneComponent.K2_SetWorldLocation` (`self.DoorPlaceOlder(Modified Scale)`) (`KismetMathLibrary.MakeVector` (.x (`self.DoorBaseLocation`)) (.y (`self.DoorBaseLocation`)) (+ (.z (`self.DoorBaseLocation`)) (* (`self.ZDelta`) _newtrack_0_2))) false false))))))))

(fn `UserConstructionScript`)