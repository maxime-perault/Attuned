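; BP_Arch is an arch that activates once when the third-person player's capsule enters its trigger, reporting to the first Door_Indicator_Base_Blueprint in the level.
; Activation plays a timeline that ramps emissive and wind parameters on the bands' dynamic material, plus the mesh's "Wind" morph target.
; The construction script creates that material with both effects at zero.
; ForceEnable calls Enable to run the same activation, bypassing the overlap and one-shot checks.
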(event `self.ArchTrigger.OnComponentBeginOverlap`
  (params (OverlappedComponent :type "PrimitiveComponent Object Reference") (OtherActor :type "Actor Object Reference") (OtherComp :type "PrimitiveComponent Object Reference") (OtherBodyIndex :type Integer) (bFromSweep :type Boolean) (SweepResult :type "HitResult Structure (by ref)"))
  (bind _dmi_bands (`self.DMI_Bands`))
  (if (and (and (== (`GameplayStatics.GetObjectClass` OtherComp) "/Script/Engine.CapsuleComponent") (== (`GameplayStatics.GetObjectClass` OtherActor) "/Game/Attuned/Characters/Player/MainCharacter/Blueprints/BP_CPPThirdPersonCharacter.BP_CPPThirdPersonCharacter_C")) (== (`self.Triggered`) false))
    (set `self.Triggered` true :!label _label)
    (bind _outactors (`GameplayStatics.GetAllActorsOfClass` "/Game/Attuned/Environment/Architectural/Giant/Door_Indicator/Door_Indicator_Base_Blueprint.Door_Indicator_Base_Blueprint_C"))
    (`/Game/Attuned/Environment/Architectural/Giant/Door_Indicator/Door_Indicator_Base_Blueprint.EnableNewArch` (`|GetArrayItem` _outactors))
    (bind (_direction _newtrack_0) (`Timeline|ActivationLerp` :!via `PlayFromStart`)
      (:`Update`
        (`MaterialInstanceDynamic.SetScalarParameterValue` _dmi_bands "Emissive_Intensity" (* _newtrack_0 3.0))
        (`MaterialInstanceDynamic.SetScalarParameterValue` _dmi_bands "Wind Intensity" _newtrack_0)
        (`SkeletalMeshComponent.SetMorphTarget` (`self.SM_Arches`) "Wind" (* _newtrack_0 2.0) true)))))

(event `Enable`
  (goto _label))

(fn `ForceEnable`
  (`self.Enable`))

(fn `UserConstructionScript`
  (bind _returnvalue (`PrimitiveComponent.CreateDynamicMaterialInstance` (`self.SM_Arches`) 1 "/Game/Attuned/Environment/Architectural/Props_01/MI_Props_01.MI_Props_01" "DMI_Bands"))
  (bind _output_get (set `self.DMI_Bands` _returnvalue))
  (`MaterialInstanceDynamic.SetScalarParameterValue` _output_get "Emissive_Intensity" 0.0)
  (`MaterialInstanceDynamic.SetScalarParameterValue` _output_get "Wind Intensity" 0.0))