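; BP_WormEye is a gameplay Blueprint that plays a camera focus moment with music when its Launch event fires.
; Launch sets a Triggered flag, starts Wwise music on itself and sets the Music state to Focus_Intro.
; It blends the player view to a child-actor camera, then after a fixed delay blends back to the player character, locking the outgoing view during both blends.
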(event `Launch`
  (if true
    (set `self.Triggered` true)
    (`AkGameplayStatics.PostEvent` "/Game/Wwise/Play_Music.Play_Music" self)
    (`AkGameplayStatics.SetState` "Music" "Focus_Intro")
    (`PlayerController.SetViewTargetWithBlend` (`GameplayStatics.GetPlayerController` 0) (`ChildActorComponent.ChildActor` (`self.BP_Camera`)) 3.0 "VTBlend_Linear" 0.0 true)
    (`KismetSystemLibrary.Delay` 3.5)
    (`PlayerController.SetViewTargetWithBlend` (`GameplayStatics.GetPlayerController` 0) (`GameplayStatics.GetPlayerCharacter` 0) 0.5 "VTBlend_Linear" 0.0 true)))

(fn `UserConstructionScript`)