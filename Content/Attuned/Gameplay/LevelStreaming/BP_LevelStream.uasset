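; BP_LevelStream is a two-trigger actor that swaps streamed levels as the player character moves between areas.
; Overlapping Enter with the character's capsule loads FirstLevel and TransiPrev and unloads SecondLevel and TransiNext; Exit does the reverse.
; IsEnter and IsExit latch the last trigger crossed, so repeat overlaps are ignored until the opposite one fires.
; All loads and unloads are non-blocking, and loaded levels become visible immediately afterwards.
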(event `self.Enter.OnComponentBeginOverlap`
  (params (OverlappedComponent :type "PrimitiveComponent Object Reference") (OtherActor :type "Actor Object Reference") (OtherComp :type "PrimitiveComponent Object Reference") (OtherBodyIndex :type Integer) (bFromSweep :type Boolean) (SweepResult :type "HitResult Structure (by ref)"))
  (if (and (and (not (`self.IsEnter`)) (== (`GameplayStatics.GetObjectClass` OtherActor) "/Game/Attuned/Characters/Player/MainCharacter/Blueprints/BP_CPPThirdPersonCharacter.BP_CPPThirdPersonCharacter_C")) (== (`GameplayStatics.GetObjectClass` OtherComp) "/Script/Engine.CapsuleComponent"))
    (set `self.IsEnter` true)
    (set `self.IsExit` false)
    (`GameplayStatics.LoadStreamLevel` (`self.FirstLevel`) true)
    (`GameplayStatics.UnloadStreamLevel` (`self.SecondLevel`))
    (`GameplayStatics.UnloadStreamLevel` (`self.TransiNext`))
    (`GameplayStatics.LoadStreamLevel` (`self.TransiPrev`) true)))

(event `self.Exit.OnComponentBeginOverlap`
  (params (OverlappedComponent :type "PrimitiveComponent Object Reference") (OtherActor :type "Actor Object Reference") (OtherComp :type "PrimitiveComponent Object Reference") (OtherBodyIndex :type Integer) (bFromSweep :type Boolean) (SweepResult :type "HitResult Structure (by ref)"))
  (if (and (and (not (`self.IsExit`)) (== (`GameplayStatics.GetObjectClass` OtherActor) "/Game/Attuned/Characters/Player/MainCharacter/Blueprints/BP_CPPThirdPersonCharacter.BP_CPPThirdPersonCharacter_C")) (== (`GameplayStatics.GetObjectClass` OtherComp) "/Script/Engine.CapsuleComponent"))
    (set `self.IsExit` true)
    (set `self.IsEnter` false)
    (`GameplayStatics.LoadStreamLevel` (`self.SecondLevel`) true)
    (`GameplayStatics.UnloadStreamLevel` (`self.FirstLevel`))
    (`GameplayStatics.LoadStreamLevel` (`self.TransiNext`) true)
    (`GameplayStatics.UnloadStreamLevel` (`self.TransiPrev`))))

(fn `UserConstructionScript`)